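; HUD Blueprint that draws the player's crosshair and an ammo readout.
; It caches the player's BaseCharacter on BeginPlay and reads its aim hit and AmmoSystem each DrawHUD.
; The crosshair follows the projected screen position of the character's hit location, falling back to screen center when no actor is hit.
; Current and inventory ammo are drawn as text near the top-left of the screen.
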(event `self.ReceiveBeginPlay`
  (bind _asbase_character (cast `/Game/Blueprints/BaseCharacter` (`GameplayStatics.GetPlayerCharacter` 0)))
  (set `self.Char` _asbase_character))

(event `self.ReceiveDrawHUD`
  (params (SizeX :type Integer) (SizeY :type Integer))
  (bind (_outhit_bblockinghit _outhit_binitialoverlap _outhit_time _outhit_distance _outhit_location _outhit_impactpoint _outhit_normal _outhit_impactnormal _outhit_physmat _outhit_hitactor) (`GameplayStatics.BreakHitResult` (`MyCharacter.OutHit` (`self.Char`))))
  (bind _ammosystem (`MyCharacter.AmmoSystem` (`self.Char`)))
  (bind _screenposition (`GameplayStatics.ProjectWorldToScreen` (`GameplayStatics.GetPlayerController` 0) _outhit_location))
  (`|ExecutionSequence`
    (:`then_0`
      ;[1 1 1] Draw Front Sight
      (`/Engine/EditorBlueprintResources/StandardMacros.IsValid` _outhit_hitactor
        (:`Is Valid`
          (`self.DrawTextureSimple` "/Game/FirstPerson/Textures/FirstPersonCrosshair.FirstPersonCrosshair" (- (`KismetMathLibrary.BreakVector2D` _screenposition) 8.0) (- (`.Y` (`KismetMathLibrary.BreakVector2D` _screenposition)) 8.0)))
        (:`Is Not Valid`
          (`self.DrawTextureSimple` "/Game/FirstPerson/Textures/FirstPersonCrosshair.FirstPersonCrosshair" (- (`KismetMathLibrary.Conv_IntToDouble` (/ SizeX 2)) 8.0) (- (`KismetMathLibrary.Conv_IntToDouble` (/ SizeY 2)) 8.0)))))
    (:`then_1`
      (`self.DrawText` (`KismetStringLibrary.Concat_StrStr` "Current Ammo : " (`KismetStringLibrary.Conv_IntToString` (`AmmoSystem.CurrentAmmo` _ammosystem)) "          Inventory Ammo : " (`KismetStringLibrary.Conv_IntToString` (`AmmoSystem.AmmoInventory` _ammosystem))) (struct :`A` 1) 100.0 (`KismetMathLibrary.Conv_IntToDouble` (/ SizeY 100)) null 1.5))))

(fn `UserConstructionScript`)